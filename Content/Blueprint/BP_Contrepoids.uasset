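; BP_Contrepoids is a counterweight puzzle actor with two linked platforms, where the heavier side sinks and the other rises.
; Overlap changes on each trigger recompute that side's weight, counting the third-person character as a fixed weight and Matryoshka actors by mesh mass.
; Tick picks low, middle (near-equal weights) or high for platform A, mirrors it for B, and eases both there with FInterpTo and swept moves.
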(event OnComponentBeginOverlap(TriggerA)
  (params (OverlappedComponent :type Primitive%20Component%20Object%20Reference) (OtherActor :type Actor%20Object%20Reference) (OtherComp :type Primitive%20Component%20Object%20Reference) (OtherBodyIndex :type Integer) (bFromSweep :type Boolean) (SweepResult :type Hit%20Result%20Structure%20%28by%20ref%29))
  (bind _total_weight (CallFunction|CalculateWeight (Variables|Default|GetTriggerA)))
  (Variables|Default|SetWeightA _total_weight))

(event OnComponentBeginOverlap(TriggerB)
  (params (OverlappedComponent :type Primitive%20Component%20Object%20Reference) (OtherActor :type Actor%20Object%20Reference) (OtherComp :type Primitive%20Component%20Object%20Reference) (OtherBodyIndex :type Integer) (bFromSweep :type Boolean) (SweepResult :type Hit%20Result%20Structure%20%28by%20ref%29))
  (bind _total_weight (CallFunction|CalculateWeight (Variables|Default|GetTriggerB)))
  (Variables|Default|SetWeightB _total_weight))

(event OnComponentEndOverlap(TriggerA)
  (params (OverlappedComponent :type Primitive%20Component%20Object%20Reference) (OtherActor :type Actor%20Object%20Reference) (OtherComp :type Primitive%20Component%20Object%20Reference) (OtherBodyIndex :type Integer))
  (bind _total_weight (CallFunction|CalculateWeight (Variables|Default|GetTriggerA)))
  (Variables|Default|SetWeightA _total_weight))

(event OnComponentEndOverlap(TriggerB)
  (params (OverlappedComponent :type Primitive%20Component%20Object%20Reference) (OtherActor :type Actor%20Object%20Reference) (OtherComp :type Primitive%20Component%20Object%20Reference) (OtherBodyIndex :type Integer))
  (bind _total_weight (CallFunction|CalculateWeight (Variables|Default|GetTriggerB)))
  (Variables|Default|SetWeightB _total_weight))

(event EventTick
  (params (DeltaSeconds :type Float%20%28single-precision%29))
  (bind _platformb (Variables|Default|GetPlatformB))
  (bind _plateforma (Variables|Default|GetPlateformA))
  (bind _relativelocation (Variables|/Script/Engine.SceneComponent|GetRelativeLocation _plateforma))
  (bind _relativelocation_2 (Variables|/Script/Engine.SceneComponent|GetRelativeLocation _platformb))
  (bind _output_get (Variables|Default|SetZ_TargetForA (Math|Float|SelectFloat 2e+02 (Math|Float|SelectFloat 0.0 4e+02 (> (Variables|Default|GetWeightA) (Variables|Default|GetWeightB))) (Math|Float|NearlyEqual(Float) (Variables|Default|GetWeightA) (Variables|Default|GetWeightB) 1.0))))
  (Transformation|SetRelativeLocation _plateforma (Math|Vector|MakeVector (.x _relativelocation) (.y _relativelocation) (Math|Interpolation|FInterpTo (.z _relativelocation) _output_get (Utilities|Time|GetWorldDeltaSeconds) 2.0)) true false)
  (bind _output_get_2 (Variables|Default|SetZ_TargetForB (- 4e+02 (Variables|Default|GetZ_TargetForA))))
  (Transformation|SetRelativeLocation _platformb (Math|Vector|MakeVector (.x _relativelocation_2) (.y _relativelocation_2) (Math|Interpolation|FInterpTo (.z _relativelocation_2) _output_get_2 (Utilities|Time|GetWorldDeltaSeconds) 2.0)) true false))

(fn ConstructionScript)

(fn CalculateWeight
  (params (TriggerZone :type Box%20Component%20Object%20Reference))
  (LocalVariables|SetLocalWeightCounter 0.0)
  (for _array_element (Collision|GetOverlappingActors TriggerZone 0 :!class /Script/Engine.PrimitiveComponent)
    (Utilities|Casting|CastToBP_ThirdPersonCharacter _array_element
      (:then
        (LocalVariables|SetLocalWeightCounter (+ (LocalVariables|GetLocalWeightCounter) 1e+02)))
      (:CastFailed
        (bind _asbp_matryoshka (Utilities|Casting|CastToBP_Matryoshka _array_element))
        (LocalVariables|SetLocalWeightCounter (+ (Physics|GetMass (Variables|/Game/Blueprint/BP_Matryoshka.BP_Matryoshka_C|GetStaticMesh _asbp_matryoshka)) (LocalVariables|GetLocalWeightCounter))))))
  (return (LocalVariables|GetLocalWeightCounter)))